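; Moving target actor that slides back and forth along the Y axis in an endless loop, starting at BeginPlay.
; It stores its spawn location as Start and an End that differs only by a hardcoded Y value.
; A forward timeline lerps between them, then a second timeline played in reverse brings it back and restarts the first.
; Points come from world location but are applied as relative location.
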(event EventBeginPlay
  (bind _returnvalue (Transformation|GetActorLocation))
  (Variables|Default|SetStart (Math|Vector|MakeVector (.x _returnvalue) (.y _returnvalue) (.z _returnvalue)))
  (Variables|Default|SetEnd (Math|Vector|MakeVector (.x _returnvalue) -1657.138672 (.z _returnvalue)))
  (bind _newtrack_0 (Timeline|Move%20forward%20Timeline PlayFromStart)
    (:Update
      (Transformation|SetActorRelativeLocation (Math|Vector|Lerp(Vector) (Variables|Default|GetStart) (Variables|Default|GetEnd) _newtrack_0)))
    (:Finished
      (bind _newtrack_0_2 (Timeline|Move%20back%20timeline ReverseFromEnd)
        (:Update
          (Transformation|SetActorRelativeLocation (Math|Vector|Lerp(Vector) (Variables|Default|GetStart) (Variables|Default|GetEnd) _newtrack_0_2)))
        (:Finished
          (Timeline|Move%20forward%20Timeline PlayFromStart))))))

(fn ConstructionScript)