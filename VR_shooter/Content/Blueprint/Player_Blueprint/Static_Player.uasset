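; Stationary first-person player for a target-shooting game that looks around, fires and ends after ten targets.
; Held fire runs rate-limited camera line traces, destroying any hit actor, showing a hit popup and updating the score widget.
; Tick-driven Delays act as one-second clocks for playtime and time between hits, averaged pairwise with the previous average.
; The tenth hit pauses and shows game over; the Reset input calls an empty function.
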(event EventBeginPlay
  (bind _returnvalue (Game|GetPlayerController 0))
  (Utilities|FlowControl|Sequence
    (:then_0
      (CallFunction|TargetScore _returnvalue))
    (:then_1
      ;[1 1 1] Adding Crosshair
      (bind _returnvalue_2 (UserInterface|CreateWidget "/Game/Widgets/Interface/Crosshair.Crosshair_C" _returnvalue))
      (UserInterface|Viewport|AddtoViewport _returnvalue_2 0))))

(event EventTick
  (params (DeltaSeconds :type Float%20%28single-precision%29))
  (Utilities|FlowControl|Sequence
    (:then_0
      ;[1 1 1] Shooting time
      (Utilities|FlowControl|Delay 1.002)
      (CallFunction|CalcShootTime))
    (:then_1
      ;[1 1 1] Playtime
      (Utilities|FlowControl|Delay 0.998)
      (CallFunction|Playtime))))

(event Input|ActionEvents|InputActionShoot
  (params (Key :type Key%20Structure :default "None"))
  (:Pressed
    ;[1 1 1] Muzzle
    (Utilities|FlowControl|DoOnce false :!label _label
      (:Completed
        (Rendering|SetVisibility (Variables|Default|GetParticleSystem) true false))))
  (:Released
    (Utilities|FlowControl|DoOnce false :!label _label_2
      (:Completed
        (Utilities|FlowControl|Sequence
          (:then_0
            (Rendering|SetVisibility (Variables|Default|GetParticleSystem) false false)
            (goto _label_2 Reset))
          (:then_1
            (goto _label Reset)))))))

(event Input|ActionEvents|InputActionReset
  (params (Key :type Key%20Structure :default "None"))
  (:Released
    (CallFunction|ResetGame)))

(event Input|AxisEvents|InputAxisLook_right
  (params (AxisValue :type Float%20%28single-precision%29))
  ;[1 1 1] Looking
  (Pawn|Input|AddControllerYawInput (* AxisValue (Variables|Default|GetTurn%20Rate) (Utilities|Time|GetWorldDeltaSeconds))))

(event Input|AxisEvents|InputAxisLook_up
  (params (AxisValue :type Float%20%28single-precision%29))
  ;[1 1 1] Looking
  (Pawn|Input|AddControllerPitchInput (* AxisValue (Variables|Default|GetTurn%20Rate) (Utilities|Time|GetWorldDeltaSeconds))))

(event Input|AxisEvents|InputAxisShoot
  (params (AxisValue :type Float%20%28single-precision%29))
  (bind _camera (Variables|Default|GetCamera))
  (bind _returnvalue (Transformation|GetWorldLocation _camera))
  ;[1 1 1] Advancded Shooting
  (if (and (== AxisValue 1.0) (Variables|Default|GetCan%20Shoot))
    (CallFunction|Shoot _returnvalue (+ _returnvalue (* (Math|Vector|GetForwardVector _camera) (Variables|Default|GetRange))))
    (Variables|Default|SetCan%20Shoot false)
    (Utilities|FlowControl|Delay 0.2)
    (Variables|Default|SetCan%20Shoot true)))

(fn ConstructionScript
  (Transformation|AttachComponentToComponent (Variables|Default|GetGun) (Variables|Default|GetCamera) "None" "KeepRelative" "KeepRelative" "KeepRelative" true))

(fn Shoot
  (params (Start%20Location :type Vector) (End%20Location :type Vector))
  (bind (_outhit _returnvalue) (Collision|LineTraceByChannel Start%20Location End%20Location "TraceTypeQuery1" true 0 "None"))
  (if _returnvalue
    (Utilities|FlowControl|Sequence
      (:then_0
        (CallFunction|UpdateTarget 1)
        (bind _returnvalue_2 (UserInterface|CreateWidget "/Game/Widgets/Popup/HIT_popup.HIT_popup_C"))
        (UserInterface|Viewport|AddtoViewport _returnvalue_2 0))
      (:then_1
        (Actor|DestroyActor (.HitActor (Collision|BreakHitResult _outhit))))
      (:then_2
        (CallFunction|UpdateAvgTime)))))

(fn TargetScore
  (params (OwningPlayer :type Player%20Controller%20Object%20Reference))
  (bind _returnvalue (UserInterface|CreateWidget "/Game/Widgets/Scorecard/Score.Score_C" OwningPlayer))
  (bind _output_get (Variables|Default|SetScore_widget _returnvalue))
  (UserInterface|Viewport|AddtoViewport _output_get 0)
  (return _returnvalue))

(fn UpdateTarget
  (params (TargetstoAdd :type Integer))
  (bind _output_get (Variables|Default|SetTargets_shot (+ TargetstoAdd (Variables|Default|GetTargets_shot))))
  (Default|UpdateTargets (Variables|Default|GetScore_widget) _output_get)
  (if (>= _output_get 10)
    (CallFunction|ShowGameOver)))

(fn ShowGameOver
  (Game|SetGamePaused true)
  (Rendering|SetVisibility (Variables|Default|GetParticleSystem) false false)
  (Viewport|RemoveAllWidgets)
  (Utilities|FlowControl|Sequence
    (:then_0
      (bind _returnvalue (UserInterface|CreateWidget "/Game/Widgets/Scorecard/Game_over.Game_over_C"))
      (UserInterface|Viewport|AddtoViewport _returnvalue 0))
    (:then_1
      (Variables|/Script/Engine.PlayerController|SetbShowMouseCursor (Game|GetPlayerController 0) true))))

(fn ResetGame)

(fn Playtime
  (Variables|Default|SetPlay_time_s (+ (Variables|Default|GetPlay_time_s) 1))
  (if (> (+ (Variables|Default|GetPlay_time_s) 1) 59)
    (Utilities|FlowControl|Sequence
      (:then_0
        (Variables|Default|SetPlay_time_s 0))
      (:then_1
        (Variables|Default|SetPlay_time_m (+ (Variables|Default|GetPlay_time_m) 1))))))

(fn CalcShootTime
  (Variables|Default|SetShoot_time_s (+ (Variables|Default|GetShoot_time_s) 1))
  (if (> (+ (Variables|Default|GetShoot_time_s) 1) 59)
    (Utilities|FlowControl|Sequence
      (:then_0
        (Variables|Default|SetShoot_time_s 0))
      (:then_1
        (Variables|Default|SetShoot_time_m (+ (Variables|Default|GetShoot_time_m) 1))))))

(fn UpdateAvgTime
  (if (and (== (Variables|Default|GetAvg_shoot_time_m) 0) (== (Variables|Default|GetAvg_shoot_time_s) 0))
    (Utilities|FlowControl|Sequence
      (:then_0
        (Variables|Default|SetAvg_shoot_time_m (Variables|Default|GetShoot_time_m))
        (Variables|Default|SetShoot_time_m 0))
      (:then_1
        (Variables|Default|SetAvg_shoot_time_s (Variables|Default|GetShoot_time_s))
        (Variables|Default|SetShoot_time_s 0)))
    (else
      (Utilities|FlowControl|Sequence
        (:then_0
          (Variables|Default|SetAvg_shoot_time_m (/ (+ (Variables|Default|GetAvg_shoot_time_m) (Variables|Default|GetShoot_time_m)) 2))
          (Variables|Default|SetShoot_time_m 0))
        (:then_1
          (Variables|Default|SetAvg_shoot_time_s (/ (+ (Variables|Default|GetAvg_shoot_time_s) (Variables|Default|GetShoot_time_s)) 2))
          (Variables|Default|SetShoot_time_s 0))))))